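; BP_Item is a respawning pickup that rolls one of six random item types on BeginPlay and each respawn, setting its duration and power.
; On overlap with an actor implementing BPI_Interaction, it passes those values through GrabItemMessage, hides, disables collision and starts a timer.
; The timer restores visibility and collision, then rerolls.
; The per-type mesh swaps in the construction script are disconnected, so the mesh does not reflect the item.
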(event OnComponentBeginOverlap(StaticMesh)
  (params (OverlappedComponent :type Primitive%20Component%20Object%20Reference) (OtherActor :type Actor%20Object%20Reference) (OtherComp :type Primitive%20Component%20Object%20Reference) (OtherBodyIndex :type Integer) (bFromSweep :type Boolean) (SweepResult :type Hit%20Result%20Structure%20%28by%20ref%29))
  (if (Utilities|DoesObjectImplementInterface OtherActor "/Game/Dev/player/BPI_Interaction.BPI_Interaction_C")
    (Class|BPIInteraction|GrabItem(Message) OtherActor (Variables|Default|GetETypeItem) (Variables|Default|GetDurer) (Variables|Default|GetPower))
    (Rendering|SetVisibility (Variables|Default|GetDefaultSceneRoot) false true)
    (Collision|SetCollisionEnabled (Variables|Default|GetStaticMesh) "NoCollision")
    (Utilities|Time|SetTimerbyEvent (delegate Custom|respawn) (Variables|Default|GetTime))))

(event Custom|respawn
  (Collision|SetCollisionEnabled (Variables|Default|GetStaticMesh) "QueryAndPhysics")
  (Rendering|SetVisibility (Variables|Default|GetDefaultSceneRoot) true true)
  (Utilities|RandomItem))

(event EventBeginPlay
  (Utilities|RandomItem))

(event Collision|EventActorBeginOverlap
  (params (OtherActor :type Actor%20Object%20Reference)))

(event EventTick
  (params (DeltaSeconds :type Float%20%28single-precision%29)))

(fn ConstructionScript)
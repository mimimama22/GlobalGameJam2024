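; BP_Projectile is a projectile that penalizes and knocks back a hit player character.
; Sphere overlap ignores the actor in RefSpawnplayer and acts only on BP_ThirdPersonCharacter.
; An unprotected target loses one Piece, floored at zero, and is launched by the projectile's velocity, added to its own, before the projectile destroys itself.
; A protected target only loses IsProtect, and the projectile is not destroyed.
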(event OnComponentBeginOverlap(Sphere)
  (params (OverlappedComponent :type Primitive%20Component%20Object%20Reference) (OtherActor :type Actor%20Object%20Reference) (OtherComp :type Primitive%20Component%20Object%20Reference) (OtherBodyIndex :type Integer) (bFromSweep :type Boolean) (SweepResult :type Hit%20Result%20Structure%20%28by%20ref%29))
  (if (!= OtherActor (Variables|Default|GetRefSpawnplayer))
    (bind _asbp_third_person_character (Utilities|Casting|CastToBP_ThirdPersonCharacter OtherActor))
    (if (not (Variables|/Game/Dev/player/Blueprints/BP_ThirdPersonCharacter.BP_ThirdPersonCharacter_C|GetIsProtect _asbp_third_person_character))
      (if (> (- (Variables|/Game/Dev/player/Blueprints/BP_ThirdPersonCharacter.BP_ThirdPersonCharacter_C|GetPiece _asbp_third_person_character) 1) 0)
        (Variables|/Game/Dev/player/Blueprints/BP_ThirdPersonCharacter.BP_ThirdPersonCharacter_C|SetPiece _asbp_third_person_character (- (Variables|/Game/Dev/player/Blueprints/BP_ThirdPersonCharacter.BP_ThirdPersonCharacter_C|GetPiece _asbp_third_person_character) 1))
        (else
          (Variables|/Game/Dev/player/Blueprints/BP_ThirdPersonCharacter.BP_ThirdPersonCharacter_C|SetPiece _asbp_third_person_character 0)))
      (Character|LaunchCharacter _asbp_third_person_character (Transformation|GetVelocity) false false)
      (Actor|DestroyActor)
      (else
        (Variables|/Game/Dev/player/Blueprints/BP_ThirdPersonCharacter.BP_ThirdPersonCharacter_C|SetIsProtect _asbp_third_person_character false)))))

(event EventBeginPlay)

(event Collision|EventActorBeginOverlap
  (params (OtherActor :type Actor%20Object%20Reference)))

(event EventTick
  (params (DeltaSeconds :type Float%20%28single-precision%29)))

(fn ConstructionScript)
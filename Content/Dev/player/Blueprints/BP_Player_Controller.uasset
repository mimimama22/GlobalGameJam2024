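; BP_Player_Controller is the player controller that sets up each of up to four local players on possessing a BP_ThirdPersonCharacter.
; Possession adds a per-player UI linked to the character, names it from GI_GGJ2024 by controller ID, and disables input.
; Outside LVL_MainMenu it also shows the WBP_DEcompte widget and writes the name to the character's TextRender.
; A separate LoadMapContext function adds the IMC_Default input mapping.
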(event EventPossess
  (params (PossessedPawn :type Pawn%20Object%20Reference))
  (bind _asbp_third_person_character (Utilities|Casting|CastToBP_ThirdPersonCharacter PossessedPawn))
  (bind _returnvalue (UserInterface|CreateWidget "/Game/Dev/UI/WBP_UI_Player.WBP_UI_Player_C" 0 _asbp_third_person_character))
  (bind _output_get (Variables|Default|SetRefUI%20Info _returnvalue))
  (bind _output_get_2 (Variables|/Game/Dev/player/Blueprints/BP_ThirdPersonCharacter.BP_ThirdPersonCharacter_C|SetRefUIPlayer _asbp_third_person_character _output_get))
  (UserInterface|Viewport|AddtoPlayerScreen _output_get_2)
  (bind _output_get_3 (Variables|Default|SetControlerID (Class|GameplayStatics|GetPlayerControllerID self)))
  (bind _asgi_ggj2024 (Utilities|Casting|CastToGI_GGJ2024 (Game|GetGameInstance)))
  (Variables|/Game/Dev/player/Blueprints/BP_ThirdPersonCharacter.BP_ThirdPersonCharacter_C|SetName _asbp_third_person_character (Utilities|Select :Index _output_get_3 :Option%200 (Variables|/Game/Dev/GI_GGJ2024.GI_GGJ2024_C|GetPlayerName1 _asgi_ggj2024) :Option%201 (Variables|/Game/Dev/GI_GGJ2024.GI_GGJ2024_C|GetPlayerName2 _asgi_ggj2024) :Option%202 (Variables|/Game/Dev/GI_GGJ2024.GI_GGJ2024_C|GetPlayerName3 _asgi_ggj2024) :Option%203 (Variables|/Game/Dev/GI_GGJ2024.GI_GGJ2024_C|GetPlayerName4 _asgi_ggj2024)))
  (Input|DisableInput _asbp_third_person_character self)
  (bind _returnvalue_2 (Game|GetCurrentLevelName true))
  (if (Utilities|Enum|NotEqual(Enum) _returnvalue_2 "LVL_MainMenu")
    (bind _returnvalue_3 (UserInterface|CreateWidget "/Game/Dev/UI/WBP_DEcompte.WBP_DEcompte_C"))
    (UserInterface|Viewport|AddtoViewport _returnvalue_3 0)
    (bind _asbp_third_person_character_2 (Utilities|Casting|CastToBP_ThirdPersonCharacter (Game|GetPlayerCharacter _output_get_3)))
    (Rendering|Components|TextRender|SetText (Variables|/Game/Dev/player/Blueprints/BP_ThirdPersonCharacter.BP_ThirdPersonCharacter_C|GetTextRender _asbp_third_person_character_2) (Variables|/Game/Dev/player/Blueprints/BP_ThirdPersonCharacter.BP_ThirdPersonCharacter_C|Getname _asbp_third_person_character_2))))

(fn ConstructionScript)

(fn LoadMapContext
  (Input|AddMappingContext (PlayerController|LocalPlayerSubsystems|GetEnhancedInputLocalPlayerSubsystem) "/Game/Dev/player/Input/IMC_Default.IMC_Default" 0 "(bIgnoreAllPressedKeysUntilRelease=True,bForceImmediately=False,bNotifyUserSettings=False)"))
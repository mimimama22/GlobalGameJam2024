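; BP_Pieces is a respawning coin pickup for the third-person character.
; When that character overlaps the Box, it calls AddCoin on the character, then hides the Cylinder and disables collision on both components.
; After the Disparition delay, it shows the coin again and restores query-only collision, reusing the same actor.
; BeginPlay also caches the player character, though the overlap logic casts the overlapping actor instead.
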(event OnComponentBeginOverlap(Box)
  (params (OverlappedComponent :type Primitive%20Component%20Object%20Reference) (OtherActor :type Actor%20Object%20Reference) (OtherComp :type Primitive%20Component%20Object%20Reference) (OtherBodyIndex :type Integer) (bFromSweep :type Boolean) (SweepResult :type Hit%20Result%20Structure%20%28by%20ref%29))
  (bind _asbp_third_person_character (Utilities|Casting|CastToBP_ThirdPersonCharacter OtherActor))
  (Default|AddCoin _asbp_third_person_character)
  (Rendering|SetVisibility (Variables|Default|GetCylinder) false false)
  (Collision|SetCollisionEnabled (Variables|Default|GetCylinder) "NoCollision")
  (Utilities|FlowControl|Delay (Variables|Default|GetDisparition))
  (Rendering|SetVisibility (Variables|Default|GetCylinder) true true)
  (Collision|SetCollisionEnabled (Variables|Default|GetCylinder) "QueryOnly"))

(event EventBeginPlay
  (bind _asbp_third_person_character (Utilities|Casting|CastToBP_ThirdPersonCharacter (Game|GetPlayerCharacter 0)))
  (Variables|Default|SetAs%20BP%20Third%20Person%20Character _asbp_third_person_character))

(event Collision|EventActorBeginOverlap
  (params (OtherActor :type Actor%20Object%20Reference)))

(event EventTick
  (params (DeltaSeconds :type Float%20%28single-precision%29)))

(fn ConstructionScript)
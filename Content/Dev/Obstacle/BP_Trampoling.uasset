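; BP_Trampoling is a trampoline obstacle that bounces the third-person player character upward when it overlaps the actor.
; On overlap it casts to BP_ThirdPersonCharacter, plays a Boing sound and stores the character reference.
; It then launches the character vertically by a Force value, doubled when the character is already falling.
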(event Collision|EventActorBeginOverlap
  (params (OtherActor :type Actor%20Object%20Reference))
  (bind _asbp_third_person_character (Utilities|Casting|CastToBP_ThirdPersonCharacter OtherActor))
  (Audio|PlaySound2D "/Game/Dev/Sound/Boing.Boing" 3.0 1.0 0.0 0 0)
  (Variables|Default|SetAs%20BP%20Third%20Person%20Character _asbp_third_person_character)
  (if (AI|Components|NavMovement|IsFalling (Variables|/Script/Engine.Character|GetCharacterMovement (Variables|Default|GetAs%20BP%20Third%20Person%20Character)))
    (Character|LaunchCharacter (Variables|Default|GetAs%20BP%20Third%20Person%20Character) (Math|Vector|MakeVector 0.0 0.0 (* (Variables|Default|GetForce) 2.0)) false false)
    (else
      (Character|LaunchCharacter (Variables|Default|GetAs%20BP%20Third%20Person%20Character) (Math|Vector|MakeVector 0.0 0.0 (Variables|Default|GetForce)) false false))))

(fn ConstructionScript)
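; BP_Obstacle2 is an obstacle Blueprint whose only logic is an elapsed-time counter shown in the UI.
; Tick calls a timer event that adds world delta seconds to Time and writes it, formatted by TimeSecondsToString, to the TextTimer of the UI_Info widget.
; The widget is reached by casting the UIInfo variable every frame.
; BeginPlay, overlap and construction logic are empty.
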(event Custom|timer
  (bind _output_get (Variables|Default|Settime (+ (Variables|Default|Gettime) (Utilities|Time|GetWorldDeltaSeconds))))
  (Rendering|Components|TextRender|SetText (Variables|/Game/Dev/UI/UI_Info.UI_Info_C|GetText_Timer (.AsUI%20Info (Utilities|Casting|CastToUI_Info (Variables|Default|GetUI_Info)))) (Utilities|Text|ToText(String) (Class|KismetStringLibrary|TimeSecondstoString _output_get))))

(event EventBeginPlay)

(event Collision|EventActorBeginOverlap
  (params (OtherActor :type Actor%20Object%20Reference)))

(event EventTick
  (params (DeltaSeconds :type Float%20%28single-precision%29))
  (CallFunction|Timer))

(fn ConstructionScript)
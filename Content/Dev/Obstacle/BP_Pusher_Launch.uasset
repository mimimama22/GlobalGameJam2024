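; Obstacle pusher that moves back and forth or along its local Y and knocks the player character away on contact.
; On BeginPlay a SetSpeed timeline, scaled by a Speed variable, continually sets the play rate of a second timeline that drives Pusher1's relative Y location.
; When a BP_ThirdPersonCharacter overlaps the Box, a punch sound plays and the character is launched along the Box's right vector times Force.
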(event OnComponentBeginOverlap(Box)
  (params (OverlappedComponent :type Primitive%20Component%20Object%20Reference) (OtherActor :type Actor%20Object%20Reference) (OtherComp :type Primitive%20Component%20Object%20Reference) (OtherBodyIndex :type Integer) (bFromSweep :type Boolean) (SweepResult :type Hit%20Result%20Structure%20%28by%20ref%29))
  (bind _asbp_third_person_character (Utilities|Casting|CastToBP_ThirdPersonCharacter OtherActor))
  (Audio|PlaySound2D "/Game/Dev/Sound/punch.punch" 1.0 1.0 0.0 0 0)
  (Character|LaunchCharacter _asbp_third_person_character (* (Math|Vector|GetRightVector (Variables|Default|GetBox)) (Variables|Default|GetForce)) false false))

(event EventBeginPlay
  (bind _speed (Timeline|SetSpeed Play)
    (:Update
      (Components|Timeline|SetPlayRate (Variables|Default|GetPusherLocation) (* _speed (Variables|Default|GetSpeed)))
      (bind _location (Timeline|PusherLocation Play)
        (:Update
          (Transformation|SetRelativeLocation (Variables|Default|GetPusher_1) (Math|Vector|MakeVector 0.0 _location 0.0) false false))))))

(fn ConstructionScript)